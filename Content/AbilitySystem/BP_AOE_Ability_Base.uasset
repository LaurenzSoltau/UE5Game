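; Base area-of-effect ability actor that finds pawns within a radius of a cast position and reports each one.
; On BeginPlay it can auto-trigger after a zero-length delay, running PreCast, which passes straight through to Cast.
; Cast runs a sphere overlap, optionally ignoring the instigator and drawing a debug sphere, then fires the OnAOEOverlap dispatcher per hit actor, leaving effects to listeners.
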(event `self.ReceiveBeginPlay`
  (if (`self.TriggerOnBeginPlay`)
    (`KismetSystemLibrary.Delay` 0.0)
    (`self.PreCast`)))

(event `PreCast`
  (`self.Cast`))

(event `Cast`
  ;[0.1094 0.1094 0.1094] Call AOEOverlap on hit targets
  (if (`self.DrawDebugSphere`)
    (`KismetSystemLibrary.DrawDebugSphere` (`self.CastPosition`) (`self.Radius`) 12 (struct :`R` 1.0 :`G` 1.0 :`B` 1.0 :`A` 1.0) 2.0 1.0))
  (bind _outactors (`KismetSystemLibrary.SphereOverlapActors` (`self.CastPosition`) (`self.Radius`) (`|MakeArray` "ObjectTypeQuery3" :!type "EObjectTypeQuery Enum") null (select `bool` (`self.IgnoreInstigator`) :`true` (`|MakeArray` (`self.GetInstigator`) :!type "Actor Object Reference"))))
  (for _array_element _outactors
    (`self.OnAOEOverlap` _array_element)))

(fn `UserConstructionScript`)