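; Base Blueprint for AOE blast abilities that plays a particle effect and sound at the cast position.
; On Cast it runs the parent logic, then spawns the blast emitter, either attached to its root to move along or free at the location.
; The actor destroys itself when the particle system finishes.
; An unset effect or sound only prints a debug message.
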(event `self.Cast`
  (`parent.Cast`)
  (`self.Spawn Blast Effect`)
  (`self.Play Blast Sound`))

(event `Spawn Blast Effect`
  ;[0.1094 0.1094 0.1094] Spawn the particle Emitter for ability
  (bind _blasteffect (`self.BlastEffect`)
    (:`then`
      (if (`self.AttachEmitter`)
        ;;[0.1094 0.1094 0.1094] Spawn Attached if should move with Character
        (bind _returnvalue (`GameplayStatics.SpawnEmitterAttached` _blasteffect (`self.DefaultSceneRoot`) "None" (`self.CastPosition`) (struct) (1.0 1.0 1.0) "KeepWorldPosition"))
        (add `ParticleSystemComponent.OnSystemFinished` _returnvalue (delegate `System Finished`))
        (else
          ;;[0.1094 0.1094 0.1094] Spawn Unattached when shouldnt move with character
          (bind _returnvalue_2 (`GameplayStatics.SpawnEmitterAtLocation` _blasteffect (`self.CastPosition`)))
          (add `ParticleSystemComponent.OnSystemFinished` _returnvalue_2 (delegate `System Finished`)))))
    (:`else`
      (`KismetSystemLibrary.PrintString` "Not Valid"))))

(event `System Finished`
  (params (PSystem :type "ParticleSystemComponent Object Reference"))
  ;[0.1094 0.1094 0.1094] Spawn the particle Emitter for ability
  ;;[0.1094 0.1094 0.1094] Spawn Attached if should move with Character
  (`self.K2_DestroyActor`))

(event `Play Blast Sound`
  ;[0.1094 0.1094 0.1094] Play Sound
  (bind _blastsound (`self.BlastSound`)
    (:`then`
      (`GameplayStatics.PlaySoundAtLocation` _blastsound (`self.CastPosition`) (struct) 1.0 1.0 0.0 null null null null))
    (:`else`
      (`KismetSystemLibrary.PrintString` "Not Valid"))))

(fn `UserConstructionScript`
  (`parent.UserConstructionScript`))