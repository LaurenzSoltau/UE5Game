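; Basic melee enemy Blueprint that chases the player and overrides its parent's Attack.
; ChasePlayer runs from BeginPlay, issuing AI MoveTo toward player controller 0, repeating three seconds after success or immediately on failure.
; Attack calls the parent, then runs a short forward debug-drawn sphere trace for pawns, leaving the result unused.
; A looping timer's event target is not shown, and the damage-response binding is unconnected.
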(event `self.ReceiveBeginPlay`
  (`KismetSystemLibrary.K2_SetTimerDelegate` (`|CreateDelegate` :!event `Attack`) 1.0 true)
  (`self.ChasePlayer`))

(event `ChasePlayer`
  (`|AIMoveTo` self (0.0 0.0 0.0) (`GameplayStatics.GetPlayerController` 0) 35.0
    (:`OnSuccess`
      (`KismetSystemLibrary.Delay` 3.0))
    (:`OnFail`
      _))
  (`self.ChasePlayer`))

(fn `Attack`
  (bind _returnvalue (`self.K2_GetActorLocation`))
  (bind (_returnvalue_roll _returnvalue_pitch _returnvalue_yaw) (`KismetMathLibrary.BreakRotator` (`self.K2_GetActorRotation`)))
  (`parent.Attack`)
  (`KismetSystemLibrary.SphereTraceSingleForObjects` :`Start` _returnvalue :`End` (+ _returnvalue (* (`KismetMathLibrary.GetForwardVector` (`KismetMathLibrary.MakeRotator` 0.0 0.0 _returnvalue_yaw)) 100.0)) :`Radius` 20.0 :`ObjectTypes` (`|MakeArray` "ObjectTypeQuery3" :!type "EObjectTypeQuery Enum") :`DrawDebugType` "ForDuration"))

(fn `UserConstructionScript`
  (`parent.UserConstructionScript`))