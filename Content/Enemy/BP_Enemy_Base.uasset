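; Base enemy Character that delegates health, healing and damage handling to its BPCDamagable component through thin wrapper functions.
; The construction script binds handlers to the component's death, damage response and blocked events.
; The event handlers knock the enemy backward along its facing when hit and print a debug message on a block, while Death destroys the actor.
; Attack is an empty stub.
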(event `Blocked`
  (`KismetSystemLibrary.PrintString` "Blocked"))

(event `DamageResponse`
  (params (DamageResponse :type "/Game/DamageSystem/E_DamageResponse Enum" :default "NewEnumerator0"))
  ;[1 1 1] Do things to the enemy after being hit
  (`self.LaunchCharacter` (* (`self.GetActorForwardVector`) -2000.0)))

(fn `Attack`)

(fn `BP_Enemy_Base_AutoGenFunc`
  (params (DamageResponse :type "/Game/DamageSystem/E_DamageResponse Enum" :default "NewEnumerator0")))

(fn `Death`
  (`self.K2_DestroyActor`))

(fn `GetCurrentHealth`
  (returns (Health :type "Float (double-precision)"))
  (return (`/Game/DamageSystem/BPC_Damagable.Health` (`self.BPC_Damagable`))))

(fn `GetMaxHealth`
  (returns (MaxHealth :type "Float (double-precision)"))
  (return (`/Game/DamageSystem/BPC_Damagable.MaxHealth` (`self.BPC_Damagable`))))

(fn `Heal`
  (params (Amount :type "Float (double-precision)"))
  (returns (NewHealth :type "Float (double-precision)"))
  (bind _newhealth (`/Game/DamageSystem/BPC_Damagable.Heal` (`self.BPC_Damagable`) Amount))
  (return _newhealth))

(fn `TakeDamage`
  (params (DamageInfo :type "/Game/DamageSystem/S_DamageInfo Structure"))
  (returns (WasDamaged :type Boolean))
  (bind _wasdamaged (`/Game/DamageSystem/BPC_Damagable.Take Damage` (`self.BPC_Damagable`) DamageInfo))
  (return _wasdamaged))

(fn `UserConstructionScript`
  (bind _bpc_damagable (`self.BPC_Damagable`))
  (add `/Game/DamageSystem/BPC_Damagable.OnDeath` _bpc_damagable (`|CreateDelegate` :!event `Death`))
  (add `/Game/DamageSystem/BPC_Damagable.OnDamageResponse` _bpc_damagable (`|CreateDelegate` :!event `DamageResponse`))
  (add `/Game/DamageSystem/BPC_Damagable.OnBlocked` _bpc_damagable (`|CreateDelegate` :!event `Blocked`)))