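; BP_Player is the player character, with Enhanced Input movement, mouse-cursor aiming and two test-keyed area abilities.
; Movement follows control rotation, while each Tick yaws the capsule toward the cursor's trace hit.
; F and H spawn whirlwind blast and lightning strike actors, whose overlap events send damage to hit actors.
; Health interface functions are stubs, except GetMaxHealth, which reads the BPCDamagable component.
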(event `self.ReceiveBeginPlay`
  ;[0.1094 0.1094 0.1094] Add Mapping Contect
  (bind _asplayer_controller (cast `PlayerController` (`self.GetController`)))
  (bind _returnvalue (pcsubsystem `EnhancedInputLocalPlayerSubsystem` _asplayer_controller))
  (`/Engine/EditorBlueprintResources/StandardMacros.IsValid` _returnvalue
    (:`Is Valid`
      (`EnhancedInputSubsystemInterface.AddMappingContext` _returnvalue "/Game/Input/IMC_Player.IMC_Player" 0 (struct))
      ;[0.1094 0.1094 0.1094] Show Mouse Cursor
      (set `PlayerController.bShowMouseCursor` true (`GameplayStatics.GetPlayerController` 0)))))

(event `EnhancedInput|/Game/Input/IA_Move`
  (params (ActionValue :type "Vector2D Structure") (ElapsedSeconds :type "Float (double-precision)") (TriggeredSeconds :type "Float (double-precision)") (InputAction :type "InputAction Object Reference" :default "/Game/Input/IA_Move.IA_Move"))
  (bind (_returnvalue_roll _returnvalue_pitch _returnvalue_yaw) (`KismetMathLibrary.BreakRotator` (`self.GetControlRotation`)))
  (bind (_returnvalue_roll_2 _returnvalue_pitch_2 _returnvalue_yaw_2) (`KismetMathLibrary.BreakRotator` (`self.GetControlRotation`)))
  ;[0.1094 0.1094 0.1094] Player Movement Input
  (:`Triggered`
    (`self.AddMovementInput` (`KismetMathLibrary.GetForwardVector` (`KismetMathLibrary.MakeRotator` 0.0 0.0 _returnvalue_yaw)) ActionValue_Y)
    (`self.AddMovementInput` (`KismetMathLibrary.GetRightVector` (`KismetMathLibrary.MakeRotator` _returnvalue_roll_2 0.0 _returnvalue_yaw_2)) ActionValue_X)))

(event `self.ReceiveTick`
  (params (DeltaSeconds :type "Float (single-precision)"))
  (`self.LookAtMouse`))

(event `LookAtMouse`
  (bind (_returnvalue_roll _returnvalue_pitch) (`KismetMathLibrary.BreakRotator` (`self.K2_GetActorRotation`)))
  (bind (_returnvalue_roll_2 _returnvalue_pitch_2 _returnvalue_yaw) (`KismetMathLibrary.BreakRotator` (`KismetMathLibrary.FindLookAtRotation` (`self.K2_GetActorLocation`) (`.Location` (`GameplayStatics.BreakHitResult` (`PlayerController.GetHitResultUnderCursorByChannel` (`GameplayStatics.GetPlayerController` 0) "TraceTypeQuery1" true))))))
  ;[0.1094 0.1094 0.1094] Look At Mouse
  (`SceneComponent.K2_SetWorldRotation` (`self.CapsuleComponent`) (`KismetMathLibrary.MakeRotator` _returnvalue_roll _returnvalue_pitch _returnvalue_yaw) false false))

(event `Key|F`
  (params (Key :type "Key Structure"))
  (:`Pressed`
    (bind _returnvalue (`|SpawnActorFromClass` "/Game/AbilitySystem/BP_AOE_Ability_Blast_Whirlwind.BP_AOE_Ability_Blast_Whirlwind_C" (`self.GetTransform`) "Undefined" "MultiplyWithRoot" null true true false true self))
    (add `/Game/AbilitySystem/BP_AOE_Ability_Base.OnAOEOverlap` _returnvalue (delegate `CustomEvent`))))

(event `CustomEvent`
  (params (Actor :type "Actor Object Reference"))
  (message `/Game/DamageSystem/BPI_Damagable.TakeDamage` Actor (make `/Game/DamageSystem/S_DamageInfo` 25.0 "NewEnumerator1" "NewEnumerator0" true)))

(event `Key|H`
  (params (Key :type "Key Structure"))
  (bind _returnvalue (`self.GetTransform`))
  (:`Pressed`
    (bind _returnvalue_2 (`|SpawnActorFromClass` "/Game/AbilitySystem/BP_AOE_Ability_LightningStrike.BP_AOE_Ability_LightningStrike_C" (`KismetMathLibrary.MakeTransform` (`KismetMathLibrary.MakeVector` (.x (.location _returnvalue)) (.y (.location _returnvalue)) (- (.z (.location _returnvalue)) 90.0)) (.rotation _returnvalue) (.scale _returnvalue)) "Undefined" "MultiplyWithRoot" null false true false true self))
    (add `/Game/AbilitySystem/BP_AOE_Ability_Base.OnAOEOverlap` _returnvalue_2 (delegate `CustomEvent`))))

(fn `GetCurrentHealth`
  (returns (Health :type "Float (double-precision)"))
  (return 0.0))

(fn `GetMaxHealth`
  (returns (MaxHealth :type "Float (double-precision)"))
  (return (`/Game/DamageSystem/BPC_Damagable.MaxHealth` (`self.BPC_Damagable`))))

(fn `Heal`
  (params (Amount :type "Float (double-precision)"))
  (returns (NewHealth :type "Float (double-precision)"))
  (return 0.0))

(fn `TakeDamage`
  (params (DamageInfo :type "/Game/DamageSystem/S_DamageInfo Structure"))
  (returns (WasDamaged :type Boolean))
  (return false))

(fn `UserConstructionScript`)