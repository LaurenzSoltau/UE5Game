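; Base area-of-effect actor for player attacks that detects pawns within a radius and reports them, without applying any effect itself.
; Trigger, optionally fired after a zero-second delay from BeginPlay, runs a one-shot sphere overlap at the actor's location, optionally ignoring the instigator and drawing a debug sphere.
; Each overlapped actor is broadcast through the OnAoeOverlap dispatcher, leaving the response to whatever binds to it.
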(event `self.ReceiveBeginPlay`
  (if (`self.TriggerOnBeginPlay`)
    (`KismetSystemLibrary.Delay` 0.0)
    (`self.Trigger`)))

(event `Trigger`
  (`self.SpawnAoeSphere`))

(event `SpawnAoeSphere`
  (if (`self.DrawDebugSphere`)
    (`KismetSystemLibrary.DrawDebugSphere` (`self.K2_GetActorLocation`) (`self.Radius`) 12 (struct :`R` 1.0 :`G` 1.0 :`B` 1.0 :`A` 1.0) 2.0 1.0))
  (bind _outactors (`KismetSystemLibrary.SphereOverlapActors` (`self.K2_GetActorLocation`) (`self.Radius`) (`|MakeArray` "ObjectTypeQuery3" :!type "EObjectTypeQuery Enum") null (select `bool` (`self.IgnoreInstigator`) :`true` (`|MakeArray` (`self.GetInstigator`) :!type "Actor Object Reference"))))
  (for _array_element _outactors
    (`self.OnAoeOverlap` _array_element)))

(fn `UserConstructionScript`)