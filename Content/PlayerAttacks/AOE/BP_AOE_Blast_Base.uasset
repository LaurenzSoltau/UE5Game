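; Base Blueprint for player AOE blast attacks, adding a particle effect and sound to the inherited AOE sphere.
; It extends the parent's SpawnAoeSphere by attaching BlastEffect to the root and playing BlastSound at the actor's location.
; The actor destroys itself when the particle system finishes.
; An unset effect or sound only prints "Not Valid", so without an effect this Blueprint never triggers that destroy.
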(event `self.SpawnAoeSphere`
  (`parent.SpawnAoeSphere`)
  (`self.Spawn Blast Effect`)
  (`self.Play Blast Sound`))

(event `Spawn Blast Effect`
  (`self.Blast Effect`
    (:`then`
      (bind _returnvalue (`GameplayStatics.SpawnEmitterAttached` (`self.Blast Effect`) (`self.DefaultSceneRoot`)))
      (add `ParticleSystemComponent.OnSystemFinished` _returnvalue (delegate `System Finished`)))
    (:`else`
      (`KismetSystemLibrary.PrintString` "Not Valid"))))

(event `System Finished`
  (params (PSystem :type "ParticleSystemComponent Object Reference"))
  (`self.K2_DestroyActor`))

(event `Play Blast Sound`
  (bind _blast_sound (`self.Blast Sound`)
    (:`then`
      (`GameplayStatics.PlaySoundAtLocation` _blast_sound (`self.K2_GetActorLocation`) (struct) 1.0 1.0 0.0 null null null null))
    (:`else`
      (`KismetSystemLibrary.PrintString` "Not Valid"))))

(fn `UserConstructionScript`
  (`parent.UserConstructionScript`))