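; Enemy spawner that places basic melee enemies around the player, at edges estimated from the viewport size.
; After a short startup delay and player check, it starts a looping timer, presumably driving SpawnEnemy.
; SpawnEnemy recalculates four player-relative edge points, picks one at random, spawns within an elongated box there and records the enemy in LivingEnemies.
; Optional debug spheres visualize the edge points.
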(event `self.ReceiveBeginPlay`
  (bind _returnvalue (`GameplayStatics.GetPlayerCharacter` 0))
  (`KismetSystemLibrary.Delay` 1.0)
  (`/Engine/EditorBlueprintResources/StandardMacros.IsValid` _returnvalue
    (:`Is Valid`
      (set `self.Player` _returnvalue)
      (`KismetSystemLibrary.K2_SetTimerDelegate` (`|CreateDelegate` :!event `SpawnEnemy`) 2.0 true))))

(fn `CalcEdgePoints`
  (bind _returnvalue_x (`KismetMathLibrary.BreakVector2D` (`WidgetLayoutLibrary.GetViewportSize`)))
  (bind (_returnvalue_x_2 _returnvalue_y) (`KismetMathLibrary.BreakVector2D` (`WidgetLayoutLibrary.GetViewportSize`)))
  (bind _returnvalue_x_3 (`KismetMathLibrary.BreakVector2D` (`WidgetLayoutLibrary.GetViewportSize`)))
  (bind (_returnvalue_x_4 _returnvalue_y_2) (`KismetMathLibrary.BreakVector2D` (`WidgetLayoutLibrary.GetViewportSize`)))
  (bind (_playerworldlocation_x _playerworldlocation_y _playerworldlocation_z) (`KismetMathLibrary.BreakVector` (`self.PlayerWorldLocation`)))
  (bind (_playerworldlocation_x_2 _playerworldlocation_y_2 _playerworldlocation_z_2) (`KismetMathLibrary.BreakVector` (`self.PlayerWorldLocation`)))
  (bind (_playerworldlocation_x_3 _playerworldlocation_y_3 _playerworldlocation_z_3) (`KismetMathLibrary.BreakVector` (`self.PlayerWorldLocation`)))
  (bind (_playerworldlocation_x_4 _playerworldlocation_y_4 _playerworldlocation_z_4) (`KismetMathLibrary.BreakVector` (`self.PlayerWorldLocation`)))
  (set `self.PlayerWorldLocation` (`SceneComponent.K2_GetComponentLocation` (`Character.CapsuleComponent` (`self.Player`))))
  (`|ExecutionSequence`
    (:`then_0`
      ;[1 1 1] Calculate Top Point
      (bind _output_get (set `self.TopPoint` (`KismetMathLibrary.MakeVector` (+ _playerworldlocation_x_2 _returnvalue_y 150.0) _playerworldlocation_y_2 _playerworldlocation_z_2))))
    (:`then_1`
      ;[1 1 1] Calculate Left Point
      (bind _output_get_2 (set `self.LeftPoint` (`KismetMathLibrary.MakeVector` _playerworldlocation_x_3 (- _playerworldlocation_y_3 _returnvalue_x_3) _playerworldlocation_z_3))))
    (:`then_2`
      ;[1 1 1] Calculate Bottom Point
      (bind _output_get_3 (set `self.BottomPoint` (`KismetMathLibrary.MakeVector` (+ (- _playerworldlocation_x_4 _returnvalue_y_2) 120.0) _playerworldlocation_y_4 _playerworldlocation_z_4))))
    (:`then_3`
      ;[1 1 1] Calculate Right Point
      (bind _output_get_4 (set `self.RightPoint` (`KismetMathLibrary.MakeVector` _playerworldlocation_x (+ _playerworldlocation_y _returnvalue_x) _playerworldlocation_z)))))
  (if (`self.drawDebugSpheres`)
    (`KismetSystemLibrary.DrawDebugSphere` _output_get 100.0 12 (struct :`R` 1.0 :`G` 0.006044 :`A` 1.0) 2.0 2.0)
    (`KismetSystemLibrary.DrawDebugSphere` _output_get_2 100.0 12 (struct :`G` 0.267204 :`B` 1.0 :`A` 1.0) 2.0 2.0)
    (`KismetSystemLibrary.DrawDebugSphere` _output_get_3 100.0 12 (struct :`R` 1.0 :`G` 0.006044 :`A` 1.0) 2.0 2.0)
    (`KismetSystemLibrary.DrawDebugSphere` _output_get_4 100.0 12 (struct :`R` 1.0 :`G` 0.006044 :`A` 1.0) 2.0 2.0)))

(fn `SpawnEnemy`
  (locals (SpawnLocation :type "Vector Structure" :default (0.0 0.0 0.0)))
  (bind (_returnvalue_x _returnvalue_y) (`KismetMathLibrary.BreakVector2D` (`WidgetLayoutLibrary.GetViewportSize`)))
  (bind _returnvalue_x_2 (`KismetMathLibrary.BreakVector2D` (`WidgetLayoutLibrary.GetViewportSize`)))
  (bind _livingenemies (`self.LivingEnemies`))
  (`self.CalcEdgePoints`)
  (switch `int` (`KismetMathLibrary.RandomInteger` 2)
    (:`0`
      (bind _returnvalue (`|SpawnActorFromClass` "/Game/Enemy/BP_Basic_Melee_Enemy.BP_Basic_Melee_Enemy_C" (`KismetMathLibrary.MakeTransform` (`KismetMathLibrary.RandomPointInBoundingBox` (`KismetArrayLibrary.Array_Random` (`|MakeArray` (`self.RightPoint`) (`self.LeftPoint`))) (`KismetMathLibrary.MakeVector` _returnvalue_x_2 30.0))) "Undefined" "MultiplyWithRoot" self null))
      (`KismetArrayLibrary.Array_Add` _livingenemies _returnvalue))
    (:`1`
      (bind _returnvalue_2 (`|SpawnActorFromClass` "/Game/Enemy/BP_Basic_Melee_Enemy.BP_Basic_Melee_Enemy_C" (`KismetMathLibrary.MakeTransform` (`KismetMathLibrary.RandomPointInBoundingBox` (`KismetArrayLibrary.Array_Random` (`|MakeArray` (`self.BottomPoint`) (`self.TopPoint`))) (`KismetMathLibrary.MakeVector` 30.0 _returnvalue_y))) "Undefined" "MultiplyWithRoot" self null))
      (`KismetArrayLibrary.Array_Add` _livingenemies _returnvalue_2))))

(fn `UserConstructionScript`)